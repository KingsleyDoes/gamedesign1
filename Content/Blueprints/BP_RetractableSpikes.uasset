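; BP_RetractableSpikes is a spike trap that retracts when a player character carrying a trap kit enters its trigger box.
; On Box overlap it casts to BP_ThirdPersonCharacterCustom, checks HasTrapKit, then plays a retract sound and the Retract timeline.
; The timeline lerps the Spikes' relative location between the Out and Retracted components' positions.
; The graph has no logic for extending the spikes again or dealing damage.
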(event `self.Box.OnComponentBeginOverlap`
  (params (OverlappedComponent :type "PrimitiveComponent Object Reference") (OtherActor :type "Actor Object Reference") (OtherComp :type "PrimitiveComponent Object Reference") (OtherBodyIndex :type Integer) (bFromSweep :type Boolean) (SweepResult :type "HitResult Structure (by ref)"))
  (bind _asbp_third_person_character_custom (cast `/Game/Blueprints/BP_ThirdPersonCharacterCustom` OtherActor))
  (if (`/Game/Blueprints/BP_ThirdPersonCharacterCustom.HasTrapKit` _asbp_third_person_character_custom)
    (`GameplayStatics.PlaySound2D` "/Game/audio/dungeonSpecific/retract_cue.retract_cue" 1.0 1.0 0.0 null null)
    (bind (_direction _newtrack_0) (`Timeline|Retract`)
      (:`Update`
        (`SceneComponent.K2_SetRelativeLocation` (`self.Spikes`) (`KismetMathLibrary.VLerp` (`SceneComponent.RelativeLocation` (`self.Out`)) (`SceneComponent.RelativeLocation` (`self.Retracted`)) _newtrack_0) false false)))))

(fn `UserConstructionScript`)