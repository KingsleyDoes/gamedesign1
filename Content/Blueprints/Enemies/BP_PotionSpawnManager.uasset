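; Manager actor that populates the level with potion ingredients at the start of play.
; On BeginPlay it gathers every BP_PotionSpawner, then spawns a BP_PotionIngredient at each spawner's location and rotation.
; Each ingredient receives a reference back to this manager, which increments a running total of ingredients as it spawns them.
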(event `self.ReceiveBeginPlay`
  (bind _outactors (`GameplayStatics.GetAllActorsOfClass` "/Game/Blueprints/Enemies/BP_PotionSpawner.BP_PotionSpawner_C"))
  (set `self.Potion Spawners` _outactors)
  (`self.Spawn Potion`))

(event `Spawn Potion`
  (for _array_element (`self.Potion Spawners`)
    (bind (_returnvalue_location _returnvalue_rotation) (`KismetMathLibrary.BreakTransform` (`SceneComponent.K2_GetComponentToWorld` (`/Game/Blueprints/Enemies/BP_PotionSpawner.DefaultSceneRoot` _array_element))))
    (bind _returnvalue (`|SpawnActorFromClass` "/Game/Blueprints/BP_PotionIngredient.BP_PotionIngredient_C" (`KismetMathLibrary.MakeTransform` _returnvalue_location _returnvalue_rotation) "Undefined" "MultiplyWithRoot" null null))
    (set `/Game/Blueprints/BP_PotionIngredient.PotionManager` self _returnvalue)
    (`/Engine/EditorBlueprintResources/StandardMacros.IncrementInt` (`self.CurrentIngredientTotal`))))

(fn `UserConstructionScript`)