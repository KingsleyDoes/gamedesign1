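; BP_Enemy is an enemy actor that dies when the player runs into it or when its body or head is struck.
; Player overlap on the capsule enables body physics, waits briefly, notifies the Manager through RemoveEnemyAndCheck, then destroys the actor.
; Any body or head hit or overlap prints a message, destroys the actor immediately and then requests a Niagara gas explosion, without notifying the Manager.
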(event `self.Capsule.OnComponentBeginOverlap`
  (params (OverlappedComponent :type "PrimitiveComponent Object Reference") (OtherActor :type "Actor Object Reference") (OtherComp :type "PrimitiveComponent Object Reference") (OtherBodyIndex :type Integer) (bFromSweep :type Boolean) (SweepResult :type "HitResult Structure (by ref)"))
  (cast `/Game/Blueprints/BP_ThirdPersonCharacterCustom` OtherActor)
  (`PrimitiveComponent.SetSimulatePhysics` (`self.Body`) true)
  (`KismetSystemLibrary.Delay` 2.0)
  (`/Game/Blueprints/Enemies/BP_EnemySpawnManager.RemoveEnemyAndCheck` (`self.Manager`))
  (`self.K2_DestroyActor`))

(event `self.Body.OnComponentHit`
  (params (HitComponent :type "PrimitiveComponent Object Reference") (OtherActor :type "Actor Object Reference") (OtherComp :type "PrimitiveComponent Object Reference") (NormalImpulse :type "Vector Structure") (Hit :type "HitResult Structure (by ref)"))
  (if true :!label _label
    (`KismetSystemLibrary.PrintString` "Oh no! I've been hit!")
    (`self.K2_DestroyActor`)
    (`NiagaraFunctionLibrary.SpawnSystemAttached` "/NiagaraFluids/Templates/Gas/2D/Systems/Grid2D_Gas_Explosion.Grid2D_Gas_Explosion" null "None" (0.0 0.0 0.0) (struct) "KeepRelativeOffset")))

(event `self.Head.OnComponentHit`
  (params (HitComponent :type "PrimitiveComponent Object Reference") (OtherActor :type "Actor Object Reference") (OtherComp :type "PrimitiveComponent Object Reference") (NormalImpulse :type "Vector Structure") (Hit :type "HitResult Structure (by ref)"))
  (goto _label))

(event `self.Body.OnComponentBeginOverlap`
  (params (OverlappedComponent :type "PrimitiveComponent Object Reference") (OtherActor :type "Actor Object Reference") (OtherComp :type "PrimitiveComponent Object Reference") (OtherBodyIndex :type Integer) (bFromSweep :type Boolean) (SweepResult :type "HitResult Structure (by ref)"))
  (goto _label))

(event `self.Head.OnComponentBeginOverlap`
  (params (OverlappedComponent :type "PrimitiveComponent Object Reference") (OtherActor :type "Actor Object Reference") (OtherComp :type "PrimitiveComponent Object Reference") (OtherBodyIndex :type Integer) (bFromSweep :type Boolean) (SweepResult :type "HitResult Structure (by ref)"))
  (goto _label))

(fn `UserConstructionScript`)