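; Floating couch actor that moves a leather sofa mesh back and forth between its Fall and Peak component positions, starting on BeginPlay.
; The Float timeline drives a vector lerp between those two relative locations to place the mesh on each update.
; When the timeline finishes, a short delay feeds a FlipFlop that alternates reverse and forward playback, looping the motion indefinitely.
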(event `self.ReceiveBeginPlay`
  (bind (_direction _newtrack_0) (`Timeline|Float` :!via `PlayFromStart` :!label _label)
    (:`Update`
      (`SceneComponent.K2_SetRelativeLocationAndRotation` :`self` (`self.SM_Classic_Leather_Sofa`) :`NewLocation` (`KismetMathLibrary.VLerp` (`SceneComponent.RelativeLocation` (`self.Fall`)) (`SceneComponent.RelativeLocation` (`self.Peak`)) _newtrack_0)))
    (:`Finished`
      (`KismetSystemLibrary.Delay` 0.2)
      (`/Engine/EditorBlueprintResources/StandardMacros.FlipFlop`
        (:`A`
          (goto _label :!via `ReverseFromEnd`))
        (:`B`
          (goto _label :!via `PlayFromStart`))))))

(fn `UserConstructionScript`)