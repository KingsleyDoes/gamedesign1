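; Lightning rod actor that becomes electrified for five seconds when anything overlaps its Box or hits its Cone.
; Both triggers add the ObjStatus.Electrified gameplay tag and turn the Cone and Cube emissive orange, then revert after a delay.
; Tick derives Activated from that tag, but an unreset DoOnce lets it become true only on the first electrification.
; GetGameplayTagContainer exposes the rod's tags.
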(event `self.ReceiveBeginPlay`
  (set `self.activated` false))

(event `self.ReceiveTick`
  (params (DeltaSeconds :type "Float (single-precision)"))
  (if (`BlueprintGameplayTagLibrary.HasTag` (`self.GameplayTags`) (struct :`TagName` "ObjStatus.Electrified"))
    (`/Engine/EditorBlueprintResources/StandardMacros.DoOnce` false
      (:`Completed`
        (set `self.activated` true)))
    (else
      (set `self.activated` false))))

(event `self.Box.OnComponentBeginOverlap`
  (params (OverlappedComponent :type "PrimitiveComponent Object Reference") (OtherActor :type "Actor Object Reference") (OtherComp :type "PrimitiveComponent Object Reference") (OtherBodyIndex :type Integer) (bFromSweep :type Boolean) (SweepResult :type "HitResult Structure (by ref)"))
  (bind _cone (`self.Cone`))
  (bind _gameplaytags (`self.GameplayTags`))
  (if true :!label _label
    (`BlueprintGameplayTagLibrary.AddGameplayTag` _gameplaytags (struct :`TagName` "ObjStatus.Electrified"))
    (`PrimitiveComponent.SetMaterial` _cone 0 "/Game/Materials/MI_EmissiveOrange.MI_EmissiveOrange")
    (`PrimitiveComponent.SetMaterial` (`self.Cube`) 0 "/Game/Materials/MI_EmissiveOrange.MI_EmissiveOrange")
    (`KismetSystemLibrary.Delay` 5.0)
    (`PrimitiveComponent.SetMaterial` _cone 0 "/Game/Materials/MI_Floor.MI_Floor")
    (`PrimitiveComponent.SetMaterial` (`self.Cube`) 0 "/Game/Materials/MI_Floor.MI_Floor")
    (`BlueprintGameplayTagLibrary.RemoveGameplayTag` _gameplaytags (struct :`TagName` "ObjStatus.Electrified"))))

(event `self.Cone.OnComponentHit`
  (params (HitComponent :type "PrimitiveComponent Object Reference") (OtherActor :type "Actor Object Reference") (OtherComp :type "PrimitiveComponent Object Reference") (NormalImpulse :type "Vector Structure") (Hit :type "HitResult Structure (by ref)"))
  (goto _label))

(fn `GetGameplayTagContainer`
  (returns (TagContainer :type "GameplayTagContainer Structure"))
  (return (`self.GameplayTags`)))

(fn `UserConstructionScript`)