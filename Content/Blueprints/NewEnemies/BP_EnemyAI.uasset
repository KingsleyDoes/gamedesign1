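; Enemy AI actor that chases and melee-attacks the player and is destroyed when damage depletes its Health.
; PawnSensing sightings set IsSeeingPlayer and start an AI move to the player, with Tick halting movement until then.
; Reaching the player triggers a CanAttack-gated palm-strike montage, with cooldown based on montage length.
; Each attack draws a debug line trace but ignores its result, always damaging the player.
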(event `self.ReceiveAnyDamage`
  (params (Damage :type "Float (single-precision)") (DamageType :type "DamageType Object Reference") (InstigatedBy :type "Controller Object Reference") (DamageCauser :type "Actor Object Reference"))
  (bind _health (`self.Health`))
  (if (> _health 0.0)
    (set `self.Health` (- _health Damage))
    (if (> (`self.Health`) 0.0)
      (`KismetSystemLibrary.PrintString` "Damn Dude")
      (else
        (`self.K2_DestroyActor`)))))

(event `self.ReceiveTick`
  (params (DeltaSeconds :type "Float (single-precision)"))
  (if (not (`self.IsSeeingPlayer`))
    (`MovementComponent.StopMovementImmediately` (`self.CharacterMovement`))))

(event `self.PawnSensing.OnSeePawn`
  (params (Pawn :type "Pawn Object Reference"))
  (set `self.IsSeeingPlayer` true)
  (`self.ChasePlayer`))

(event `ChasePlayer`
  (set `self.CanAttack` true)
  (if (`self.IsSeeingPlayer`)
    (`|AIMoveTo` self (0.0 0.0 0.0) (`GameplayStatics.GetPlayerCharacter` 0) 90.0
      (:`OnSuccess`
        (if (`self.CanAttack`)
          (`self.AttackPlayer`))))
    (else
      (set `self.IsSeeingPlayer` false))))

(event `AttackPlayer`
  (set `self.CanAttack` false)
  (bind _returnvalue (`self.PlayAnimMontage` "/Game/Blueprints/NewEnemies/Animations/Paired_CounterPunch_PalmStrike_Att_Quinn_Montage.Paired_CounterPunch_PalmStrike_Att_Quinn_Montage"))
  (bind _outhit (`KismetSystemLibrary.LineTraceSingle` :`Start` (`SceneComponent.GetSocketLocation` (`self.StartAttack`) "None") :`End` (`SceneComponent.GetSocketLocation` (`self.EndAttack`) "None") :`TraceChannel` "TraceTypeQuery1" :`DrawDebugType` "ForDuration"))
  (`GameplayStatics.ApplyDamage` (`GameplayStatics.GetPlayerCharacter` 0) 2.0)
  (`KismetSystemLibrary.Delay` (+ _returnvalue 0.5))
  (set `self.CanAttack` true))

(fn `UserConstructionScript`)