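; BP_UIPickup is an actor that shows its own display name in a widget component as a pickup label.
; On BeginPlay it creates a W_UIPickup widget, assigns it to the component and fills the ItemName text.
; A self-calling event with a short delay keeps rotating the widget toward the player camera, billboarding it without using Tick.
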(event `self.ReceiveBeginPlay`
  (bind _returnvalue (`|CreateWidget` "/Game/Widgets/W_UIPickup.W_UIPickup_C"))
  (`WidgetComponent.SetWidget` (`self.Widget`) _returnvalue)
  (set `TextBlock.Text` (`KismetTextLibrary.Conv_StringToText` (`KismetSystemLibrary.GetDisplayName` self)) (`/Game/Widgets/W_UIPickup.ItemName` _returnvalue))
  (`self.RotateToFace`))

(event `RotateToFace`
  (bind _widget (`self.Widget`))
  (`SceneComponent.K2_SetWorldRotation` _widget (`KismetMathLibrary.FindLookAtRotation` (`SceneComponent.K2_GetComponentLocation` _widget) (`SceneComponent.K2_GetComponentLocation` (`PlayerCameraManager.TransformComponent` (`GameplayStatics.GetPlayerCameraManager` 0)))) false false)
  (`KismetSystemLibrary.Delay` 0.1)
  (`self.RotateToFace`))

(fn `UserConstructionScript`)